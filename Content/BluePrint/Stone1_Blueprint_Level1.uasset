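; Level 1 stone actor that rotates about its yaw axis one step per call to E_PreesedMovement, in a twelve-step cycle.
; A nested chain of twelve boolean flags selects which of twelve timelines plays from the start, each driving the actor's rotation.
; Each timeline update sets its own flag and clears the following one, with the last clearing the first so the sequence wraps around.
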(event Custom|E_PreesedMovement
  (if (Variables|Default|GetPreesed_1)
    (if (Variables|Default|GetPreesed_2)
      (if (Variables|Default|GetPreesed_3)
        (if (Variables|Default|GetPreesed_4)
          (if (Variables|Default|GetPreesed_5)
            (if (Variables|Default|GetPreesed_6)
              (if (Variables|Default|GetPreesed_7)
                (if (Variables|Default|GetPreesed_8)
                  (if (Variables|Default|GetPreesed_9)
                    (if (Variables|Default|GetPreesed_10)
                      (if (Variables|Default|GetPreesed_11)
                        (if (not (Variables|Default|GetPreesed_12))
                          (bind _newtrack_0 (Timeline|Timeline_12 PlayFromStart)
                            (:Update
                              (Transformation|SetActorRotation (Math|Rotator|MakeRotator 0.0 0.0 _newtrack_0))
                              (Variables|Default|SetPreesed_12 true)
                              (Variables|Default|SetPreesed_1 false))))
                        (else
                          (bind _newtrack_0_2 (Timeline|Timeline_11 PlayFromStart)
                            (:Update
                              (Transformation|SetActorRotation (Math|Rotator|MakeRotator 0.0 0.0 _newtrack_0_2))
                              (Variables|Default|SetPreesed_11 true)
                              (Variables|Default|SetPreesed_12 false)))))
                      (else
                        (bind _newtrack_0_3 (Timeline|Timeline_10 PlayFromStart)
                          (:Update
                            (Transformation|SetActorRotation (Math|Rotator|MakeRotator 0.0 0.0 _newtrack_0_3))
                            (Variables|Default|SetPreesed_10 true)
                            (Variables|Default|SetPreesed_11 false)))))
                    (else
                      (bind _newtrack_0_4 (Timeline|Timeline_9 PlayFromStart)
                        (:Update
                          (Transformation|SetActorRotation (Math|Rotator|MakeRotator 0.0 0.0 _newtrack_0_4))
                          (Variables|Default|SetPreesed_9 true)
                          (Variables|Default|SetPreesed_10 false)))))
                  (else
                    (bind _newtrack_0_5 (Timeline|Timeline_8 PlayFromStart)
                      (:Update
                        (Transformation|SetActorRotation (Math|Rotator|MakeRotator 0.0 0.0 _newtrack_0_5))
                        (Variables|Default|SetPreesed_8 true)
                        (Variables|Default|SetPreesed_9 false)))))
                (else
                  (bind _newtrack_0_6 (Timeline|Timeline_7 PlayFromStart)
                    (:Update
                      (Transformation|SetActorRotation (Math|Rotator|MakeRotator 0.0 0.0 _newtrack_0_6))
                      (Variables|Default|SetPreesed_7 true)
                      (Variables|Default|SetPreesed_8 false)))))
              (else
                (bind _newtrack_0_7 (Timeline|Timeline_6 PlayFromStart)
                  (:Update
                    (Transformation|SetActorRotation (Math|Rotator|MakeRotator 0.0 0.0 _newtrack_0_7))
                    (Variables|Default|SetPreesed_6 true)
                    (Variables|Default|SetPreesed_7 false)))))
            (else
              (bind _newtrack_0_8 (Timeline|Timeline_5 PlayFromStart)
                (:Update
                  (Transformation|SetActorRotation (Math|Rotator|MakeRotator 0.0 0.0 _newtrack_0_8))
                  (Variables|Default|SetPreesed_5 true)
                  (Variables|Default|SetPreesed_6 false)))))
          (else
            (bind _newtrack_0_9 (Timeline|Timeline_4 PlayFromStart)
              (:Update
                (Transformation|SetActorRotation (Math|Rotator|MakeRotator 0.0 0.0 _newtrack_0_9))
                (Variables|Default|SetPreesed_4 true)
                (Variables|Default|SetPreesed_5 false)))))
        (else
          (bind _newtrack_0_10 (Timeline|Timeline_3 PlayFromStart)
            (:Update
              (Transformation|SetActorRotation (Math|Rotator|MakeRotator 0.0 0.0 _newtrack_0_10))
              (Variables|Default|SetPreesed_3 true)
              (Variables|Default|SetPreesed_4 false)))))
      (else
        (bind _newtrack_0_11 (Timeline|Timeline_2 PlayFromStart)
          (:Update
            (Transformation|SetActorRotation (Math|Rotator|MakeRotator 0.0 0.0 _newtrack_0_11))
            (Variables|Default|SetPreesed_2 true)
            (Variables|Default|SetPreesed_3 false)))))
    (else
      (bind _newtrack_0_12 (Timeline|Timeline_1 PlayFromStart)
        (:Update
          (Transformation|SetActorRotation (Math|Rotator|MakeRotator 0.0 0.0 _newtrack_0_12))
          (Variables|Default|SetPreesed_1 true)
          (Variables|Default|SetPreesed_2 false))))))

(fn ConstructionScript)