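; PictureStoneTrigger1 is a match-level stone actor that turns through a four-step rotation cycle each time its pressed-movement event fires.
; Four chained booleans select one of four timelines, which drives the actor's yaw from its track.
; Each timeline update sets its own step flag and clears another, so the sequence wraps back to the first rotation after the fourth.
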(event Custom|E_PreesedMovement
  (if (Variables|Default|GetPreesed_1)
    (if (Variables|Default|GetPreesed_2)
      (if (Variables|Default|GetPreesed_3)
        (if (not (Variables|Default|GetPreesed_4))
          (bind _newtrack_0 (Timeline|Timeline_3 PlayFromStart)
            (:Update
              (Transformation|SetActorRotation (Math|Rotator|MakeRotator 0.0 0.0 _newtrack_0))
              (Variables|Default|SetPreesed_4 true)
              (Variables|Default|SetPreesed_1 false))))
        (else
          (bind _newtrack_0_2 (Timeline|Timeline_2 PlayFromStart)
            (:Update
              (Transformation|SetActorRotation (Math|Rotator|MakeRotator 0.0 0.0 _newtrack_0_2))
              (Variables|Default|SetPreesed_3 true)
              (Variables|Default|SetPreesed_4 false)))))
      (else
        (bind _newtrack_0_3 (Timeline|Timeline_1 PlayFromStart)
          (:Update
            (Transformation|SetActorRotation (Math|Rotator|MakeRotator 0.0 0.0 _newtrack_0_3))
            (Variables|Default|SetPreesed_2 true)
            (Variables|Default|SetPreesed_3 false)))))
    (else
      (bind _newtrack_0_4 (Timeline|Timeline_0 PlayFromStart)
        (:Update
          (Transformation|SetActorRotation (Math|Rotator|MakeRotator 0.0 0.0 _newtrack_0_4))
          (Variables|Default|SetPreesed_1 true)
          (Variables|Default|SetPreesed_2 false))))))

(fn ConstructionScript)