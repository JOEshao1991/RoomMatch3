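; Sun, Earth and Moon Blueprint that animates orbital rotation with a shadow track component, apparently to demonstrate shadows between the bodies.
; Nested timelines started on BeginPlay set the yaw of Earth2StaticMesh, ShadowTrack and Moon, while the innermost update also hides ShadowTrack in game.
; ShadowTrack's end overlap resets Earth1StaticMesh to BasicShapeMaterial.
; Its begin-overlap check on Sphere2 does nothing, and the LightOn_2 material swap is disconnected.
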(event OnComponentBeginOverlap(ShadowTrack)
  (params (OverlappedComponent :type Primitive%20Component%20Object%20Reference) (OtherActor :type Actor%20Object%20Reference) (OtherComp :type Primitive%20Component%20Object%20Reference) (OtherBodyIndex :type Integer) (bFromSweep :type Boolean) (SweepResult :type Hit%20Result%20Structure%20%28by%20ref%29))
  (if (Collision|IsOverlappingActor (Variables|Default|GetSphere2) OtherActor :!class /Script/Engine.PrimitiveComponent)
    _))

(event OnComponentEndOverlap(ShadowTrack)
  (params (OverlappedComponent :type Primitive%20Component%20Object%20Reference) (OtherActor :type Actor%20Object%20Reference) (OtherComp :type Primitive%20Component%20Object%20Reference) (OtherBodyIndex :type Integer))
  (if true
    (Rendering|Material|SetMaterial (Variables|Default|GetEarth1_StaticMesh) 0 "/Game/Materials/BasicShapeMaterial.BasicShapeMaterial")))

(event EventBeginPlay
  (bind _newtrack_0 (Timeline|Sun_Earth Play)
    (:Update
      (Transformation|SetRelativeRotation (Variables|Default|GetEarth2_StaticMesh) (Math|Rotator|MakeRotator 0.0 0.0 _newtrack_0) false false)
      (bind _newtrack_0_2 (Timeline|Timeline_0 Play)
        (:Update
          (Transformation|SetRelativeRotation (Variables|Default|GetShadowTrack) (Math|Rotator|MakeRotator 0.0 0.0 _newtrack_0_2) false false)
          (bind _newtrack_1 (Timeline|Earth_Moon Play)
            (:Update
              (Transformation|SetRelativeRotation (Variables|Default|GetMoon) (Math|Rotator|MakeRotator 0.0 0.0 _newtrack_1) false false)
              (Development|SetHiddeninGame (Variables|Default|GetShadowTrack) true false))))))))

(fn ConstructionScript)