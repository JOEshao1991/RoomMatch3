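; Gear stone controller Blueprint that spins gear meshes and tracks whether the player can use it.
; Sphere overlap by the ThirdPersonCharacter toggles input and the EKeyEnable flag.
; The Rotation event, with no caller in this graph, plays a timeline driving three meshes' rotation, two using the negated value.
; Each timeline update also requests the gear sound and sets EKeyDown, which a half-second delay clears.
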(event OnComponentBeginOverlap(Sphere)
  (params (OverlappedComponent :type Primitive%20Component%20Object%20Reference) (OtherActor :type Actor%20Object%20Reference) (OtherComp :type Primitive%20Component%20Object%20Reference) (OtherBodyIndex :type Integer) (bFromSweep :type Boolean) (SweepResult :type Hit%20Result%20Structure%20%28by%20ref%29))
  (Utilities|Casting|CastToThirdPersonCharacter OtherActor)
  (Input|EnableInput (Game|GetPlayerController 0))
  (Variables|Default|SetE_Key_Enable true))

(event OnComponentEndOverlap(Sphere)
  (params (OverlappedComponent :type Primitive%20Component%20Object%20Reference) (OtherActor :type Actor%20Object%20Reference) (OtherComp :type Primitive%20Component%20Object%20Reference) (OtherBodyIndex :type Integer))
  (Utilities|Casting|CastToThirdPersonCharacter OtherActor)
  (Input|DisableInput (Game|GetPlayerController 0))
  (Variables|Default|SetE_Key_Enable false))

(event Custom|Rotation
  (bind _staticmesh1 (Variables|Default|GetStaticMesh1))
  (bind _returnvalue (Transformation|GetRelativeTransform _staticmesh1))
  (bind _newtrack_2 (Timeline|Timeline_0 PlayFromStart)
    (:Update
      (Variables|Default|SetE_KeyDown true)
      (Transformation|SetRelativeRotation (Variables|Default|Getgear_StaticMesh) (Math|Rotator|MakeRotator 0.0 _newtrack_2 0.0) false false)
      (Transformation|SetRelativeRotation _staticmesh1 (Math|Rotator|MakeRotator (.roll (.rotation _returnvalue)) (.pitch (.rotation _returnvalue)) (* _newtrack_2 -1.0)) false false)
      (Transformation|SetRelativeRotation (Variables|Default|GetStaticMesh) (Math|Rotator|MakeRotator 0.0 (* _newtrack_2 -1.0) 0.0) false false)
      (Audio|PlaySound2D "/Game/Pops/Gear.Gear")
      (Utilities|FlowControl|Delay 0.5)
      (Variables|Default|SetE_KeyDown false))))

(fn ConstructionScript)